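; BP_Coding is a practice Actor Blueprint that demonstrates adding two numbers through a function and a custom event.
; On BeginPlay it prints the result of the MyAdd function, then calls the MyAdd2 event, which prints the sum of its inputs itself.
; A NewMacro macro is present but unused, and the overlap, tick and end-play events do nothing.
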(event `MyAdd2`
  (params (a :type Integer) (b :type Integer))
  (`KismetSystemLibrary.PrintString` (`KismetStringLibrary.Conv_IntToString` (+ a b))))

(event `self.ReceiveBeginPlay`
  (`KismetSystemLibrary.PrintString` (`KismetStringLibrary.Conv_IntToString` (`self.MyAdd` 10 20)))
  (`self.MyAdd2` 0))

(event `self.ReceiveEndPlay`
  (params (EndPlayReason :type "EEndPlayReason Enum" :default "Destroyed")))

(fn `MyAdd`
  (params (a :type Integer) (b :type Integer))
  (returns (result :type Integer))
  (return (+ a b)))

(fn `UserConstructionScript`)