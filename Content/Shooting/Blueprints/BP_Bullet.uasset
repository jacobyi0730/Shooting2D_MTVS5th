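; BP_Bullet is a projectile actor that flies straight ahead and destroys enemies it hits.
; Each Tick, Translate moves it along its forward vector by Speed scaled by delta time, without sweeping.
; On overlap with a BP_Enemy, it destroys both that enemy and itself and plays a quiet 2D explosion sound.
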(event `self.ReceiveActorBeginOverlap`
  (params (OtherActor :type "Actor Object Reference"))
  (bind _asbp_enemy (cast `/Game/Shooting/Blueprints/BP_Enemy` OtherActor))
  (`self.K2_DestroyActor` _asbp_enemy)
  (`self.K2_DestroyActor`)
  (`GameplayStatics.PlaySound2D` "/Game/Shooting/Sound/Audio_Explosion.Audio_Explosion" 0.2 1.0 0.0 null null))

(event `self.ReceiveTick`
  (params (DeltaSeconds :type "Float (single-precision)"))
  (`self.Translate` (`self.Speed`)))

(fn `Translate`
  (params (Speed :type "Float (double-precision)"))
  (`self.K2_SetActorLocation` (+ (`self.K2_GetActorLocation`) (* (`self.GetActorForwardVector`) Speed (`GameplayStatics.GetWorldDeltaSeconds`)))))

(fn `UserConstructionScript`)