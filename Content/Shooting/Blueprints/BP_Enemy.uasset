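; Enemy actor for a shooting game that flies in a straight line and ends the game on touching the player.
; On BeginPlay it has a 30% chance to aim at the player's position, otherwise keeping its forward vector.
; Tick moves it along that fixed direction without sweeping.
; Player overlap destroys both, pauses and shows the game-over widget, while EndPlay always spawns a Niagara explosion.
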(event `self.ReceiveActorBeginOverlap`
  (params (OtherActor :type "Actor Object Reference"))
  (bind _asbp_player (cast `/Game/Shooting/Blueprints/BP_Player` OtherActor))
  (`self.K2_DestroyActor` _asbp_player)
  (`self.K2_DestroyActor`)
  (bind _returnvalue (`|CreateWidget` "/Game/Shooting/Blueprints/UI/WBP_GameOver.WBP_GameOver_C"))
  (`UserWidget.AddToViewport` _returnvalue 0)
  (`GameplayStatics.SetGamePaused` true)
  (`WidgetBlueprintLibrary.SetInputMode_UIOnlyEx` (`GameplayStatics.GetPlayerController` 0) null)
  (set `PlayerController.bShowMouseCursor` true (`GameplayStatics.GetPlayerController` 0)))

(event `self.ReceiveBeginPlay`
  (if (< (`KismetMathLibrary.RandomIntegerInRange` 0 9) 3)
    (bind _output_get (set `self.Direction` (`KismetMathLibrary.Normal` (- (`self.K2_GetActorLocation` (`GameplayStatics.GetPlayerPawn` 0)) (`self.K2_GetActorLocation`)))))
    (`self.K2_SetActorRotation` (`KismetMathLibrary.MakeRotFromXZ` _output_get (`self.GetActorUpVector`)))
    (else
      (set `self.Direction` (`self.GetActorForwardVector`)))))

(event `self.ReceiveTick`
  (params (DeltaSeconds :type "Float (single-precision)"))
  (`self.Translate` (`self.Speed`) (`self.Direction`)))

(event `self.ReceiveEndPlay`
  (params (EndPlayReason :type "EEndPlayReason Enum" :default "Destroyed"))
  (`NiagaraFunctionLibrary.SpawnSystemAtLocation` "/Game/Shooting/Materials/NS_Explosion.NS_Explosion" (`self.K2_GetActorLocation`)))

(fn `Translate`
  (params (Speed :type "Float (double-precision)") (Direction :type "Vector Structure"))
  (`self.K2_SetActorLocation` (+ (`self.K2_GetActorLocation`) (* Direction Speed (`GameplayStatics.GetWorldDeltaSeconds`)))))

(fn `UserConstructionScript`)