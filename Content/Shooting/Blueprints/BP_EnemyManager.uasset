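; BP_EnemyManager is an enemy spawner that keeps creating BP_Enemy actors at its Arrow component's transform.
; After a one-second delay at BeginPlay, it picks a random interval between MinTime and MaxTime and sets an event timer.
; Each timer firing spawns an enemy and re-arms the timer with a new random interval.
; An older Tick-based timer is left disconnected, alongside a Test function that prints a greeting.
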(event `SetMakeTime`
  (set `self.MakeTime` (`KismetMathLibrary.RandomFloatInRange` (`self.MinTime`) (`self.MaxTime`))))

(event `self.ReceiveBeginPlay`
  (`KismetSystemLibrary.Delay` 1.0)
  (`self.SetMakeTime` :!label _label)
  (`KismetSystemLibrary.K2_SetTimerDelegate` (delegate `MakeEnemy`) (`self.MakeTime`)))

(event `MakeEnemy`
  (`|SpawnActorFromClass` "/Game/Shooting/Blueprints/BP_Enemy.BP_Enemy_C" (`SceneComponent.K2_GetComponentToWorld` (`self.Arrow`)) "Undefined" "MultiplyWithRoot" null null)
  (goto _label))

(event `self.ReceiveTick`
  (params (DeltaSeconds :type "Float (single-precision)")))

(fn `Test`
  (`KismetSystemLibrary.PrintString` "Hello"))

(fn `UserConstructionScript`)