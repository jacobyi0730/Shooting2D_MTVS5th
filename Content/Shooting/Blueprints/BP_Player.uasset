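; BP_Player is the player actor for a shooting game, moving along its own right and up axes.
; BeginPlay applies a fixed 45-degree rotation, so movement follows the tilted local axes.
; Each Tick combines the Horizontal and Vertical values into a normalized direction, scaled by Speed and delta time for frame-rate-independent movement without sweep collision.
; The graph does not set those two axis values, and the overlap event is empty.
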(event `self.ReceiveBeginPlay`
  (`self.K2_SetActorRotation` (struct :`Roll` 45.0)))

(event `self.ReceiveTick`
  (params (DeltaSeconds :type "Float (single-precision)"))
  ; 이동을 하고싶다.
  (`self.K2_SetActorLocation` (+ (`self.K2_GetActorLocation`) (* (`KismetMathLibrary.Normal` (+ (* (`self.GetActorRightVector`) (`self.GetInputAxisValue`)) (* (`self.GetActorUpVector`) (`self.GetInputAxisValue`)))) (`self.Speed`) (`GameplayStatics.GetWorldDeltaSeconds`)))))

(fn `UserConstructionScript`)